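; Animated human character actor (Maximo) whose skeletal mesh animation can be paused and resumed.
; On BeginPlay it jumps the animation to a random position within the first few seconds, varying the start pose per instance.
; Freeze and Unfreeze events stop and restore the mesh's play rate.
; When Debug is set, BeginPlay and Tick draw a red box around the actor's bounds, including child actors.
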(event `self.ReceiveBeginPlay`
  (bind (_origin _boxextent) (`self.GetActorBounds` false true))
  (`SkeletalMeshComponent.SetPosition` (`self.SkeletalMesh1`) (`KismetMathLibrary.RandomFloatInRange` 0.0 3.0) true)
  (if (`self.debug`)
    (`KismetSystemLibrary.DrawDebugBox` _origin _boxextent (struct :`R` 1.0 :`A` 1.0) (struct) 0.1 10.0 :!label _label)))

(event `self.ReceiveTick`
  (params (DeltaSeconds :type "Float (single-precision)"))
  (if (`self.debug`)
    (goto _label)))

(event `/Game/Blueprints/Interfaces/FreezeInterface.freeze`
  (`SkeletalMeshComponent.SetPlayRate` (`self.SkeletalMesh1`) 0.0))

(event `/Game/Blueprints/Interfaces/FreezeInterface.unfreeze`
  (`SkeletalMeshComponent.SetPlayRate` (`self.SkeletalMesh1`) 1.0))

(fn `UserConstructionScript`)