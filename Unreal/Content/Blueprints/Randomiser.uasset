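; Scene randomiser that varies time of day, ocean, sky and spawned props around a computer vision pawn, which it aligns to CameraRef at startup.
; On a timer or forced trigger, it respawns random amounts of Spawneables inside SpawnBox.
; Placement avoids listed actors and earlier spawns using padded bounds and class extents cached at BeginPlay.
; It picks a random Y, subtracts blocked X intervals and samples the remaining space, retrying on failure.
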(event EventBeginPlay
  (Development|PrintString (Utilities|String|ToString(Vector2d) (Viewport|GetViewportSize)))
  (for _array_element (Variables|Default|GetAvoid)
    (Utilities|Array|Add (Variables|Default|GetAvoidAreas) (Math|Box2D|MakeBox2D (CallFunction|ToXY (.Min (CallFunction|GetBoxMinMax (.Origin (Collision|GetActorBounds _array_element false false)) (+ (.BoxExtent (Collision|GetActorBounds _array_element false false)) (Variables|Default|GetAvoidMargin))))) (CallFunction|ToXY (.Max (CallFunction|GetBoxMinMax (.Origin (Collision|GetActorBounds _array_element false false)) (+ (.BoxExtent (Collision|GetActorBounds _array_element false false)) (Variables|Default|GetAvoidMargin))))))))
  (for _array_element_2 (Variables|Default|GetSpawneables)
    (for _array_element_3 (.blueprintclass _array_element_2)
      (if (Class|KismetMathLibrary|IsZero2D (.overrideextents _array_element_2))
        (bind _returnvalue (Game|SpawnActorfromClass _array_element_3 (Math|Transform|MakeTransform "0, 0, 0" "0, 0, 0" "1,1,1") "Undefined" 0 0))
        (Utilities|Map|Add (Variables|Default|GetBPClassBoundsMap) _array_element_3 (Math|Vector2D|MakeVector2D (.x (.BoxExtent (Collision|GetActorBounds _returnvalue false true))) (.y (.BoxExtent (Collision|GetActorBounds _returnvalue false true)))))
        (Actor|DestroyActor _returnvalue)))))

(event Collision|EventActorBeginOverlap
  (params (OtherActor :type Actor%20Object%20Reference)))

(event EventTick
  (params (DeltaSeconds :type Float%20%28single-precision%29))
  (if (Variables|Default|GetColdStart)
    (if (!= (Variables|Reference|GetCameraRef) 0)
      (bind _returnvalue (Actor|GetActorOfClass "/AirSim/Blueprints/BP_ComputerVisionPawn.BP_ComputerVisionPawn_C"))
      (Transformation|SetActorTransform _returnvalue (Transformation|GetActorTransform (Variables|Reference|GetCameraRef))))
    (Variables|Default|SetColdStart false))
  (if (Variables|Default|GetautoPopulate)
    (Variables|Default|Settime (+ (Variables|Default|Gettime) DeltaSeconds)))
  (if (or (>= (Variables|Default|Gettime) (Variables|Default|GetautoInterval)) (Variables|Default|GetforcePopulate))
    (Variables|Default|SetforcePopulate false)
    (Variables|Default|Settime 0.0)
    (CallFunction|Randomise)))

(event EventRandomise
  (bind _timemanager (Variables|Reference|GetTimeManager))
  (bind _hourrange (Variables|Param|GethourRange))
  (Variables|/Script/TimePlugin.TimeManager|SetCurrentLocalTime _timemanager (Utilities|Struct|MakeTimeDate (.year (Variables|/Script/TimePlugin.TimeManager|GetCurrentLocalTime _timemanager)) (.month (Variables|/Script/TimePlugin.TimeManager|GetCurrentLocalTime _timemanager)) (.day (Variables|/Script/TimePlugin.TimeManager|GetCurrentLocalTime _timemanager)) (Math|Random|RandomIntegerinRange (Math|Float|Truncate (.min _hourrange)) (Math|Float|Truncate (.max _hourrange))) (.minute (Variables|/Script/TimePlugin.TimeManager|GetCurrentLocalTime _timemanager)) (.second (Variables|/Script/TimePlugin.TimeManager|GetCurrentLocalTime _timemanager)) (.millisecond (Variables|/Script/TimePlugin.TimeManager|GetCurrentLocalTime _timemanager))))
  (CallFunction|RandomiseOceanParams)
  (CallFunction|RandomiseSkyParams)
  (CallFunction|Repopulate))

(fn ConstructionScript)

(fn Repopulate
  (bind _avoidareas (Variables|Default|GetAvoidAreas))
  ;[1 1 1] Clean up previous actors
  (for _array_element (Variables|Default|GetSpawnedActors)
    (Actor|DestroyActor _array_element)
    (Utilities|Array|RemoveIndex _avoidareas (- (Utilities|Array|Length _avoidareas) 1)))
  (Utilities|Array|Clear (Variables|Default|GetSpawnedActors))
  (for _array_element_2 (Variables|Default|GetSpawneables)
    (Variables|Default|SetzVal (.zvalue _array_element_2))
    (Variables|Default|Setscale (.scale _array_element_2))
    (Variables|Default|SetoverrideExtents (.overrideextents _array_element_2))
    (bind _output_get (Variables|Default|SettempRand (Math|Random|RandomInteger (+ (.amount _array_element_2) 1))))
    (if (> _output_get 0)
      (for _index (range 0 _output_get)
        ;[1 1 1] Choose random blueprint if there is a list of blueprints in the spawn details
        (Variables|Default|SetSpawnClass (Utilities|Array|Get(acopy) (.blueprintclass _array_element_2) (select (> (Utilities|Array|Length (.blueprintclass _array_element_2)) 1) (Math|Random|RandomInteger (Utilities|Array|Length (.blueprintclass _array_element_2))) 0)))
        (Variables|Default|SetrandomRot (Math|Random|RandomRotator false))
        (bind (_randomcoord _success) (CallFunction|GetRandomXYCoord :!label _label))
        (if _success
          (LocalVariables|Setpos (Math|Vector|MakeVector (.x (+ (Math|Vector|MakeVector (.x _randomcoord) (.y _randomcoord) (Variables|Default|GetzVal)) (Transformation|GetWorldLocation (Variables|Default|GetDefaultSceneRoot)))) (.y (+ (Math|Vector|MakeVector (.x _randomcoord) (.y _randomcoord) (Variables|Default|GetzVal)) (Transformation|GetWorldLocation (Variables|Default|GetDefaultSceneRoot)))) (.z (+ (Math|Vector|MakeVector (.x _randomcoord) (.y _randomcoord) (Variables|Default|GetzVal)) (Transformation|GetWorldLocation (Variables|Default|GetDefaultSceneRoot))))))
          (bind _returnvalue (Game|SpawnActorfromClass (Variables|Default|GetSpawnClass) (Math|Transform|MakeTransform (LocalVariables|Getpos) (Math|Rotator|MakeRotator 0.0 0.0 (.yaw (Variables|Default|GetrandomRot))) (+ (Math|Vector|VectorZero) (Variables|Default|Getscale))) "Undefined" 0 0))
          (Utilities|Array|AddUnique (Variables|Default|GetSpawnedActors) _returnvalue)
          ;[1 1 1] Adds bounding box of newly created instance to blacklist areas with some margin included
          (Utilities|Array|Add (Variables|Default|GetAvoidAreas) (Math|Box2D|MakeBox2D (CallFunction|ToXY (.Min (CallFunction|GetBoxMinMax (.Origin (Collision|GetActorBounds _returnvalue false false)) (+ (select (Class|KismetMathLibrary|IsZero2D (Variables|Default|GetoverrideExtents)) (.BoxExtent (Collision|GetActorBounds _returnvalue false false)) (Math|Vector|MakeVector (.X (Math|Vector2D|BreakVector2D (Variables|Default|GetoverrideExtents))) (.Y (Math|Vector2D|BreakVector2D (Variables|Default|GetoverrideExtents))) 1e+02)) (Variables|Default|GetInstanceMargin))))) (CallFunction|ToXY (.Max (CallFunction|GetBoxMinMax (.Origin (Collision|GetActorBounds _returnvalue false false)) (+ (select (Class|KismetMathLibrary|IsZero2D (Variables|Default|GetoverrideExtents)) (.BoxExtent (Collision|GetActorBounds _returnvalue false false)) (Math|Vector|MakeVector (.X (Math|Vector2D|BreakVector2D (Variables|Default|GetoverrideExtents))) (.Y (Math|Vector2D|BreakVector2D (Variables|Default|GetoverrideExtents))) 1e+02)) (Variables|Default|GetInstanceMargin)))))))
          (else
            (bind _result (Math|Integer|IncrementInt (LocalVariables|Gettries))
              (:%20%20
                (if (>= _result 100)
                  (Development|PrintString "Scene is too full")
                  (return)
                  (else
                    (Development|PrintString "Failed allocation")
                    (goto _label)))))))))))

(fn GetBoxMinMax
  (params (Origin :type Vector) (Extents :type Vector))
  (return (Math|Vector|MakeVector (- (.x Origin) (.x Extents)) (- (.y Origin) (.y Extents)) (- (.z Origin) (.z Extents))) (Math|Vector|MakeVector (+ (.x Origin) (.x Extents)) (+ (.y Origin) (.y Extents)) (+ (.z Origin) (.z Extents)))))

(fn ToXY
  (params (Vector :type Vector))
  (return (Math|Vector2D|MakeVector2D (.x Vector) (.y Vector))))

(fn GetBoxArea
  (params (min :type Vector%202D%20Structure) (max :type Vector%202D%20Structure))
  (return (* (- (.x max) (.x min)) (- (.y max) (.y min)))))

(fn GetRandomArea
  (params (fullArea :type Float%20%28single-precision%29) (avoidAreas :type Array%20of%20Floats%20%28single-precision%29))
  (LocalVariables|SetrandomArea fullArea)
  (for _array_element avoidAreas
    (LocalVariables|SetrandomArea (- (LocalVariables|GetrandomArea) _array_element)))
  (return (LocalVariables|GetrandomArea)))

(fn GetAvoidAreas
  (for _array_element (Variables|Default|GetAvoid)
    (Utilities|Array|Add (LocalVariables|Getareas) (CallFunction|GetBoxArea (CallFunction|ToXY (.Min (CallFunction|GetBoxMinMax (.Origin (Collision|GetActorBounds _array_element false false)) (.BoxExtent (Collision|GetActorBounds _array_element false false))))) (CallFunction|ToXY (.Max (CallFunction|GetBoxMinMax (.Origin (Collision|GetActorBounds _array_element false false)) (.BoxExtent (Collision|GetActorBounds _array_element false false))))))))
  (return (LocalVariables|Getareas)))

(fn FromRandomtoWorld
  (params (randomFloat :type Float%20%28single-precision%29))
  (bind _returnvalue (- 0.0 1.0))
  (bind _output_get (LocalVariables|Sety (Math|Conversions|ToFloat(Integer) (Math|Float|Truncate (/ randomFloat _returnvalue)))))
  (LocalVariables|Setx (Math|Float|%(Float) randomFloat _returnvalue))
  (if (> _output_get (.y (CallFunction|ToXY (.Min (CallFunction|GetBoxMinMax (.Origin (Collision|GetActorBounds (stale _array_element) false false)) (.BoxExtent (Collision|GetActorBounds (stale _array_element) false false)))))))
    _))

(fn GetRandomXYCoord
  (bind _bpclassboundsmap (Variables|Default|GetBPClassBoundsMap))
  (bind _overrideextents (Variables|Default|GetoverrideExtents))
  (bind _scale (Variables|Default|Getscale))
  (bind _defaultsceneroot (Variables|Default|GetDefaultSceneRoot))
  (bind _spawnbox (Variables|Default|GetSpawnBox))
  (bind _spawnbox_2 (Variables|Default|GetSpawnBox))
  (bind _spawnbox_3 (Variables|Default|GetSpawnBox))
  (bind _rangelist (LocalVariables|GetrangeList))
  (bind _spawnclass (Variables|Default|GetSpawnClass))
  (bind _rangelist_2 (LocalVariables|GetrangeList))
  (bind _value (Utilities|Map|Find _bpclassboundsmap _spawnclass))
  (bind _returnvalue (Class|KismetMathLibrary|IsZero2D _overrideextents))
  (bind _returnvalue_2 (Transformation|GetWorldLocation _defaultsceneroot))
  (bind _xyvector (CallFunction|ToXY _returnvalue_2))
  (bind _returnvalue_3 (select _returnvalue _value _overrideextents))
  (bind _returnvalue_4 (* _returnvalue_3 _scale))
  (bind _output_get (LocalVariables|Setwidth (- (.x (.max _spawnbox_2)) (.x (.min _spawnbox_2)))))
  (bind _output_get_2 (LocalVariables|Setheight (- (.y (.max _spawnbox_2)) (.y (.min _spawnbox_2)))))
  (LocalVariables|SetinitialRange (Math|Vector2D|MakeVector2D 0.0 _output_get))
  (LocalVariables|Sety (Math|Random|RandomFloatinRange 0.0 _output_get_2))
  (for _array_element (Variables|Default|GetAvoidAreas)
    (LocalVariables|SetavoidBox (Math|Box2D|MakeBox2D (Math|Vector2D|MakeVector2D (.x (- (- (.min _array_element) (.min _spawnbox)) _xyvector)) (.y (- (- (.min _array_element) (.min _spawnbox)) _xyvector))) (Math|Vector2D|MakeVector2D (.x (- (- (.max _array_element) (.min _spawnbox)) _xyvector)) (.y (- (- (.max _array_element) (.min _spawnbox)) _xyvector)))))
    (if _returnvalue
      (bind _returnvalue_5 (Game|SpawnActorfromClass (Variables|Default|GetSpawnClass) (Math|Transform|MakeTransform "0, 0, 0" (Variables|Default|GetrandomRot) "1,1,1") "Undefined" 0 0))
      (Actor|DestroyActor _returnvalue_5))
    (if (and (< (LocalVariables|Gety) (.y (+ (.max (LocalVariables|GetavoidBox)) _returnvalue_4))) (> (LocalVariables|Gety) (.y (- (.min (LocalVariables|GetavoidBox)) _returnvalue_4))))
      (Utilities|Array|Add (LocalVariables|GetexclList) (Utilities|Struct|MakeRange (select (< (.x (- (.min (LocalVariables|GetavoidBox)) _returnvalue_4)) 0.0) 0.0 (.x (- (.min (LocalVariables|GetavoidBox)) _returnvalue_4))) (select (> (.x (+ (.max (LocalVariables|GetavoidBox)) _returnvalue_4)) (LocalVariables|Getwidth)) (LocalVariables|Getwidth) (.x (+ (.max (LocalVariables|GetavoidBox)) _returnvalue_4)))))))
  (Utilities|Array|Add (LocalVariables|GetrangeList) (Utilities|Struct|MakeRange (.x (LocalVariables|GetinitialRange)) (.y (LocalVariables|GetinitialRange))))
  (for _array_element_2 (LocalVariables|GetexclList)
    (for (_array_element_3 _array_index) _rangelist_2
      (switch Utilities|FlowControl|Switch|SwitchonInsideCriteria (CallFunction|GetInsideCriteriaAtoB _array_element_2 _array_element_3)
        (:NewEnumerator0
          (if (Utilities|Enum|Equal(Enum) (CallFunction|GetInsideCriteriaAtoB _array_element_3 _array_element_2) "NewEnumerator3")
            (Utilities|Array|RemoveIndex _rangelist_2 _array_index :!label _label)))
        (:NewEnumerator1
          (Utilities|Array|Add _rangelist_2 (Utilities|Struct|MakeRange (.min (Utilities|Struct|BreakRange _array_element_3)) (.min (Utilities|Struct|BreakRange _array_element_2))))
          (goto _label))
        (:NewEnumerator2
          (Utilities|Array|Add _rangelist_2 (Utilities|Struct|MakeRange (.max (Utilities|Struct|BreakRange _array_element_2)) (.max (Utilities|Struct|BreakRange _array_element_3))))
          (goto _label))
        (:NewEnumerator3
          (Utilities|Array|Add _rangelist_2 (Utilities|Struct|MakeRange (.min (Utilities|Struct|BreakRange _array_element_3)) (.min (Utilities|Struct|BreakRange _array_element_2))))
          (Utilities|Array|Add _rangelist_2 (Utilities|Struct|MakeRange (.max (Utilities|Struct|BreakRange _array_element_2)) (.max (Utilities|Struct|BreakRange _array_element_3))))
          (goto _label)))))
  ;[1 1 1] Calculate the available x-space for the chosen y-value to choose randomly from
  (LocalVariables|SetrandomSize 0.0)
  (for _array_element_4 (LocalVariables|GetrangeList)
    (LocalVariables|SetrandomSize (+ (- (.max _array_element_4) (.min _array_element_4)) (LocalVariables|GetrandomSize))))
  (while (!= (Utilities|Array|Length (LocalVariables|GetrangeList)) 0)
    (LocalVariables|Setlowest 1e+07)
    (LocalVariables|SetlowestIdx -1)
    (for (_array_element_5 _array_index_2) _rangelist
      (if (< (.min _array_element_5) (LocalVariables|Getlowest))
        (LocalVariables|Setlowest (.min _array_element_5))
        (LocalVariables|SetlowestIdx _array_index_2)))
    (Utilities|Array|Add (LocalVariables|GetorderedRangeList) (Utilities|Array|Get(acopy) _rangelist (LocalVariables|GetlowestIdx)))
    (Utilities|Array|RemoveIndex _rangelist (LocalVariables|GetlowestIdx)))
  (if (<= (LocalVariables|GetrandomSize) 1.0)
    ;[1 1 1] No place to spawn. Return success = false
    (return "" false)
    (else
      (LocalVariables|Setx (Math|Random|RandomFloatinRange 0.0 (LocalVariables|GetrandomSize)))
      (for _array_element_6 (LocalVariables|GetorderedRangeList)
        (bind _output_get_3 (LocalVariables|Setx (- (LocalVariables|Getx) (- (.max _array_element_6) (.min _array_element_6)))))
        (if (< _output_get_3 0.0)
          (bind _output_get_4 (LocalVariables|Setx (+ (.max _array_element_6) _output_get_3)))
          (return (Math|Vector2D|MakeVector2D (+ _output_get_4 (.x (.min _spawnbox_3))) (+ (LocalVariables|Gety) (.y (.min _spawnbox_3)))) true))))))

(fn HasIntersection
  (params (Range%20A :type Range%20Structure) (Range%20B :type Range%20Structure))
  (return (not (or (> (.min Range%20A) (.max Range%20B)) (< (.max Range%20A) (.min Range%20B))))))

(fn GetInsideCriteriaAtoB
  (params (Range%20A :type Range%20Structure) (Range%20B :type Range%20Structure))
  (bind _returnvalue (<= (.max Range%20A) (.max Range%20B)))
  (bind _returnvalue_2 (<= (.min Range%20A) (.max Range%20B)))
  (bind _returnvalue_3 (>= (.max Range%20A) (.min Range%20B)))
  (bind _returnvalue_4 (>= (.min Range%20A) (.min Range%20B)))
  (bind _returnvalue_5 (and _returnvalue_4 _returnvalue_2))
  (bind _returnvalue_6 (and _returnvalue_3 _returnvalue))
  (bind _returnvalue_7 (not _returnvalue_5))
  (bind _returnvalue_8 (not _returnvalue_6))
  (if (and _returnvalue_5 _returnvalue_6)
    (return "NewEnumerator3")
    (elif (and _returnvalue_5 _returnvalue_8)
      (return "NewEnumerator1")
      (elif (and _returnvalue_7 _returnvalue_6)
        (return "NewEnumerator2")
        (elif (and _returnvalue_7 _returnvalue_8)
          (return "NewEnumerator0"))))))

(fn RandomiseOceanParams
  (bind _seacolorhuerange (Variables|Param|GetseaColorHueRange))
  (bind _seacolorsaturationrange (Variables|Param|GetseaColorSaturationRange))
  (bind _seaopacityrange (Variables|Param|GetseaOpacityRange))
  (bind _ocean (Variables|Reference|GetOcean))
  (bind _searoughnessrange (Variables|Param|GetseaRoughnessRange))
  (Class|KismetMathLibrary|LinearColorSetfromHSV (Variables|/OceanPlugin/Ocean/BP_OceanManager.BP_OceanManager_C|GetBaseColorLight (Variables|Reference|GetOcean)) (Math|Random|RandomFloatinRange (.min _seacolorhuerange) (.max _seacolorhuerange)) (Math|Random|RandomFloatinRange (.min _seacolorsaturationrange) (.max _seacolorsaturationrange)) 0.01 1.0)
  (Variables|/OceanPlugin/Ocean/BP_OceanManager.BP_OceanManager_C|SetOpacity _ocean (Math|Random|RandomFloatinRange (.min _seaopacityrange) (.max _seaopacityrange)))
  (Variables|/OceanPlugin/Ocean/BP_OceanManager.BP_OceanManager_C|SetRoughness _ocean (Math|Random|RandomFloatinRange (.min _searoughnessrange) (.max _searoughnessrange)))
  (Default|SetDisplayParameters (Variables|Reference|GetOcean))
  (return))

(fn RandomiseSkyParams
  (bind _sky (Variables|Reference|GetSky))
  (bind _fogdensityrange (Variables|Param|GetfogDensityRange))
  (bind _sunlightintenserange (Variables|Param|GetsunLightIntenseRange))
  (Variables|/SkyPlugin/BP_Sky.BP_Sky_C|SetHeightFogDensity _sky (select (<= (Math|Random|RandomFloat) (Variables|Param|GetfogChance)) (Math|Random|RandomFloatinRange (.min _fogdensityrange) (.max _fogdensityrange)) 0.0))
  (Variables|/SkyPlugin/BP_Sky.BP_Sky_C|SetSunLightIntensity _sky (Math|Random|RandomFloatinRange (.min _sunlightintenserange) (.max _sunlightintenserange)))
  (Default|SetSkyParameters (Variables|Reference|GetSky) false))