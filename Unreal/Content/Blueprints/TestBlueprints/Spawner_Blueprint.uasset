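; Test spawner actor that periodically spawns random primitive shapes near itself.
; Tick accumulates delta time and, every five seconds, spawns a random cube, sphere, cone or cylinder actor class, then resets the counter.
; Each spawn is offset by a random unit vector from the root, with randomized rotation and non-uniform scale.
; Leftover radius-based circular placement math is unconnected.
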(event `self.ReceiveTick`
  (params (DeltaSeconds :type "Float (single-precision)"))
  (bind (_returnvalue_x _returnvalue_y _returnvalue_z) (`KismetMathLibrary.BreakVector` (* (`KismetMathLibrary.Vector_GetAbs` (`KismetMathLibrary.RandomUnitVector`)) 360.0)))
  (bind _output_get (set `self.Counter` (+ DeltaSeconds (`self.Counter`))))
  (if (> _output_get 5.0)
    (`|SpawnActorFromClass` (`KismetArrayLibrary.Array_Random` (`|MakeArray` "/Game/Blueprints/TestBlueprints/Cube_spawn.Cube_spawn_C" "/Game/Blueprints/TestBlueprints/Sphere_spawn.Sphere_spawn_C" "/Game/Blueprints/TestBlueprints/Cone_spawn.Cone_spawn_C" "/Game/Blueprints/TestBlueprints/Cylinder_spawn.Cylinder_spawn_C" :!type "Actor Class Reference")) (`KismetMathLibrary.MakeTransform` (+ (`KismetMathLibrary.RandomUnitVector`) (`SceneComponent.K2_GetComponentLocation` (`self.DefaultSceneRoot`))) (`KismetMathLibrary.MakeRotator` _returnvalue_x _returnvalue_y _returnvalue_z) (+ (* (`KismetMathLibrary.Vector_GetAbs` (`KismetMathLibrary.RandomUnitVector`)) 4.0) 0.5)) "Undefined" "OverrideRootScale" null null)
    (set `self.Counter` 0.0)))

(fn `UserConstructionScript`)